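; BP_Environment is a scrolling scenery piece that moves along X and recycles itself with a new random look.
; Tick shifts the root by FloatSpeed divided by DeltaSeconds, then resets X to zero once it reaches the far limit.
; BeginPlay and each reset call InitializingALocation, which draws random garbage, rock, tree, house and bush meshes from data tables.
; The Move event called at BeginPlay is empty.
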(event Custom|Event%20Move)

(event EventBeginPlay
  (CallFunction|InitializingALocation)
  (CallFunction|EventMove))

(event Collision|EventActorBeginOverlap
  (params (OtherActor :type Actor%20Object%20Reference)))

(event EventTick
  (params (DeltaSeconds :type Float%20%28single-precision%29))
  (bind _defaultsceneroot (Variables|Default|GetDefaultSceneRoot))
  (bind _returnvalue (Transformation|GetWorldLocation _defaultsceneroot))
  (Transformation|SetRelativeLocation _defaultsceneroot (Math|Vector|MakeVector (+ (/ (Variables|Default|GetFloat_Speed) DeltaSeconds) (.x _returnvalue)) (.y _returnvalue) (.z _returnvalue)) false false)
  (if (>= (.x _returnvalue) 6e+03)
    (Transformation|SetRelativeLocation _defaultsceneroot (Math|Vector|MakeVector 0.0 (.y _returnvalue) (.z _returnvalue)) false false)
    (CallFunction|InitializingALocation)))

(fn ConstructionScript)

(fn InitializingALocation
  (bind _outrownames (DataTable|GetDataTableRowNames (Variables|Default|GetDT_GarbageList)))
  (bind _returnvalue (Utilities|GetDataTableRow "/Game/Project/BluePrintsAndOther/DateTable/DT_GarbageList.DT_GarbageList" (Utilities|Array|Get(acopy) _outrownames (Math|Random|RandomIntegerinRange 0 2)))
    (:then
      (Components|StaticMesh|SetStaticMesh (Variables|Default|GetGarbage) (.mesh _returnvalue))
      (bind _outrownames_2 (DataTable|GetDataTableRowNames (Variables|Default|GetDT_RockList)))
      (bind _returnvalue_2 (Utilities|GetDataTableRow "/Game/Project/BluePrintsAndOther/DateTable/DT_RockList.DT_RockList" (Utilities|Array|Get(acopy) _outrownames_2 (Math|Random|RandomIntegerinRange 0 2)))
        (:then
          (Components|StaticMesh|SetStaticMesh (Variables|Default|GetRock) (.mesh _returnvalue_2))
          (bind _outrownames_3 (DataTable|GetDataTableRowNames (Variables|Default|GetDT_TreesList)))
          (bind _returnvalue_3 (Utilities|GetDataTableRow "/Game/Project/BluePrintsAndOther/DateTable/DT_TreesList.DT_TreesList" (Utilities|Array|Get(acopy) _outrownames_3 (Math|Random|RandomIntegerinRange 0 2)))
            (:then
              (Components|StaticMesh|SetStaticMesh (Variables|Default|GetTrees) (.mesh _returnvalue_3))
              (bind _outrownames_4 (DataTable|GetDataTableRowNames (Variables|Default|GetDT_HouseList)))
              (bind _returnvalue_4 (Utilities|GetDataTableRow "/Game/Project/BluePrintsAndOther/DateTable/DT_HouseList.DT_HouseList" (Utilities|Array|Get(acopy) _outrownames_4 (Math|Random|RandomIntegerinRange 0 2)))
                (:then
                  (Components|StaticMesh|SetStaticMesh (Variables|Default|GetHouse) (.mesh _returnvalue_4))
                  (bind _outrownames_5 (DataTable|GetDataTableRowNames (Variables|Default|GetDT_BushList)))
                  (bind _returnvalue_5 (Utilities|GetDataTableRow "/Game/Project/BluePrintsAndOther/DateTable/DT_BushList.DT_BushList" (Utilities|Array|Get(acopy) _outrownames_5 (Math|Random|RandomIntegerinRange 0 2)))
                    (:then
                      (Components|StaticMesh|SetStaticMesh (Variables|Default|GetBush) (.mesh _returnvalue_5)))))))))))))