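; BP_Environment is a scrolling scenery actor that moves along X and loops back with a newly randomized look.
; Tick advances the root by FloatSpeed divided by DeltaSeconds, making movement frame-rate dependent, and wraps it past an X threshold.
; At BeginPlay and each wrap, InitializingALocation chains random DataTable picks for garbage, rock, house and bush meshes, then rarely shows a shop.
; The tree randomization is left unconnected.
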(event EventBeginPlay
  (CallFunction|InitializingALocation))

(event Collision|EventActorBeginOverlap
  (params (OtherActor :type Actor%20Object%20Reference)))

(event EventTick
  (params (DeltaSeconds :type Float%20%28single-precision%29))
  (bind _defaultsceneroot (Variables|Default|GetDefaultSceneRoot))
  (bind _returnvalue (Transformation|GetWorldLocation _defaultsceneroot))
  (Transformation|SetRelativeLocation _defaultsceneroot (Math|Vector|MakeVector (+ (/ (Variables|Default|GetFloat_Speed) DeltaSeconds) (.x _returnvalue)) (.y _returnvalue) (.z _returnvalue)) false false)
  (if (>= (.x _returnvalue) 1.3e+04)
    (Transformation|SetRelativeLocation _defaultsceneroot (Math|Vector|MakeVector -7e+03 (.y _returnvalue) (.z _returnvalue)) false false)
    (CallFunction|InitializingALocation)))

(fn ConstructionScript)

(fn InitializingALocation
  (bind _shop (Variables|Default|GetShop))
  (bind _outrownames (DataTable|GetDataTableRowNames (Variables|Default|GetDT_GarbageList)))
  (bind _returnvalue (Utilities|GetDataTableRow "/Game/DataTable/DT_GarbageList.DT_GarbageList" (Utilities|Array|Get(acopy) _outrownames (Math|Random|RandomIntegerinRange 0 2)))
    (:then
      (Components|StaticMesh|SetStaticMesh (Variables|Default|GetGarbage) (.mesh _returnvalue))
      (bind _outrownames_2 (DataTable|GetDataTableRowNames (Variables|Default|GetDT_RockList)))
      (bind _returnvalue_2 (Utilities|GetDataTableRow "/Game/DataTable/DT_RockList.DT_RockList" (Utilities|Array|Get(acopy) _outrownames_2 (Math|Random|RandomIntegerinRange 0 2)))
        (:then
          (Components|StaticMesh|SetStaticMesh (Variables|Default|GetRock) (.mesh _returnvalue_2))
          (bind _outrownames_3 (DataTable|GetDataTableRowNames (Variables|Default|GetDT_HouseList)))
          (bind _returnvalue_3 (Utilities|GetDataTableRow "/Game/DataTable/DT_HouseList.DT_HouseList" (Utilities|Array|Get(acopy) _outrownames_3 (Math|Random|RandomIntegerinRange 0 2)))
            (:then
              (Components|StaticMesh|SetStaticMesh (Variables|Default|GetHouse) (.mesh _returnvalue_3))
              (bind _outrownames_4 (DataTable|GetDataTableRowNames (Variables|Default|GetDT_BushList)))
              (bind _returnvalue_4 (Utilities|GetDataTableRow "/Game/DataTable/DT_BushList.DT_BushList" (Utilities|Array|Get(acopy) _outrownames_4 (Math|Random|RandomIntegerinRange 0 2)))
                (:then
                  (Components|StaticMesh|SetStaticMesh (Variables|Default|GetBush) (.mesh _returnvalue_4))
                  (if (== (Math|Random|RandomIntegerinRange 0 100) 50)
                    (Components|StaticMesh|SetStaticMesh _shop "/Game/Modeles/Shop_Bild/StaticMeshes/Shop_Bild.Shop_Bild")
                    (else
                      (Components|StaticMesh|SetStaticMesh _shop 0))))))))))))