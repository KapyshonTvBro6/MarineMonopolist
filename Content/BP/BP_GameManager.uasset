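; BP_GameManager is a manager Blueprint that links money changes and the fisherman actor to the game's UI widget.
; The UI reference is stored through GetUI, which acts as a setter despite its name.
; After short startup delays, BeginPlay binds the money-changed event, then passes itself and the found BP_Fisherman to the UI.
; Each money change forwards the new amount to the UI for display.
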(event Custom|OnMoneyChanged_Event
  (params (NewMoneyAmount :type Integer))
  (Default|UpdateMone (Variables|Default|GetUI) NewMoneyAmount))

(event EventBeginPlay
  (Utilities|FlowControl|Delay 1.0)
  (EventDispatchers|BindEventtoOnMoneyChanged (delegate Custom|OnMoneyChanged_Event))
  (Utilities|FlowControl|Delay 0.2)
  (bind _returnvalue (Actor|GetActorOfClass "/Game/BP/BP_Fisherman.BP_Fisherman_C"))
  (Default|GetGameObjects (Variables|Default|GetUI) self _returnvalue))

(fn ConstructionScript)

(fn GetUI
  (params (WBP_UI :type WBP%20UI%20Object%20Reference))
  (Variables|Default|SetUI WBP_UI))